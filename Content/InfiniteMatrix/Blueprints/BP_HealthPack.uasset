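; BP_HealthPack is a health pickup that restores one point of player health, capped at a maximum of ten.
; Healing runs only when the HealthPack component is hit by BP_Player, after which the pack destroys itself.
; A player overlapping TriggerZone destroys the pack without healing, while any BP_Shooting actor overlapping HealthPack is destroyed and leaves the pack intact.
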(event `self.TriggerZone.OnComponentBeginOverlap`
  (params (OverlappedComponent :type "PrimitiveComponent Object Reference") (OtherActor :type "Actor Object Reference") (OtherComp :type "PrimitiveComponent Object Reference") (OtherBodyIndex :type Integer) (bFromSweep :type Boolean) (SweepResult :type "HitResult Structure (by ref)"))
  (cast `/Game/InfiniteMatrix/Blueprints/BP_Player` OtherActor)
  (`self.K2_DestroyActor`))

(event `self.HealthPack.OnComponentBeginOverlap`
  (params (OverlappedComponent :type "PrimitiveComponent Object Reference") (OtherActor :type "Actor Object Reference") (OtherComp :type "PrimitiveComponent Object Reference") (OtherBodyIndex :type Integer) (bFromSweep :type Boolean) (SweepResult :type "HitResult Structure (by ref)"))
  (bind _asbp_shooting (cast `/Game/InfiniteMatrix/Blueprints/BP_Shooting` OtherActor))
  (`self.K2_DestroyActor` _asbp_shooting))

(event `self.HealthPack.OnComponentHit`
  (params (HitComponent :type "PrimitiveComponent Object Reference") (OtherActor :type "Actor Object Reference") (OtherComp :type "PrimitiveComponent Object Reference") (NormalImpulse :type "Vector Structure") (Hit :type "HitResult Structure (by ref)"))
  (bind _asbp_player (cast `/Game/InfiniteMatrix/Blueprints/BP_Player` OtherActor))
  (bind _returnvalue (+ (`/Game/InfiniteMatrix/Blueprints/BP_Player.Health` _asbp_player) 1))
  (if (> _returnvalue 10)
    (set `/Game/InfiniteMatrix/Blueprints/BP_Player.Health` 10 _asbp_player)
    (else
      (set `/Game/InfiniteMatrix/Blueprints/BP_Player.Health` _returnvalue _asbp_player)))
  (`self.K2_DestroyActor`))

(fn `UserConstructionScript`)